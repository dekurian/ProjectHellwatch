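; Audio wrapper Blueprint that adds start, stop, pause and resume control with position memory to its Audio component.
; While audio plays, Tick accumulates delta time into a playback counter and wraps it at the sound's duration, which keeps the position valid for looping.
; Pause is emulated by saving the counter and stopping the audio, and resume plays again from that saved time.
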(event EventTick
  (params (DeltaSeconds :type Float%20%28single-precision%29))
  (if (Audio|Components|Audio|IsPlaying (Variables|Default|GetAudio))
    (Variables|Default|SetPlaybackCounter (+ (Variables|Default|GetPlaybackCounter) (Utilities|Time|GetWorldDeltaSeconds)))
    (if (>= (Variables|Default|GetPlaybackCounter) (Variables|Default|GetDuration))
      (Variables|Default|SetPlaybackCounter (- (Variables|Default|GetPlaybackCounter) (Variables|Default|GetDuration))))))

(fn ConstructionScript)

(fn StartSound
  (bind _audio (Variables|Default|GetAudio))
  (Variables|Default|SetDuration (Variables|/Script/Engine.SoundBase|GetDuration (Variables|/Script/Engine.AudioComponent|GetSound _audio)))
  (Variables|Default|SetPlaybackCounter 0.0)
  (Audio|Components|Audio|Play _audio 0.0))

(fn StopSound
  (Audio|Components|Audio|Stop (Variables|Default|GetAudio)))

(fn ResumeSound
  (Audio|Components|Audio|Play (Variables|Default|GetAudio) (Variables|Default|GetPlaybackTime)))

(fn PauseSound
  (Variables|Default|SetPlaybackTime (Variables|Default|GetPlaybackCounter))
  (Audio|Components|Audio|Stop (Variables|Default|GetAudio)))