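; BP_TB_SpawnSwitch is an overlap trigger that activates switches and spawn areas and can start a sequence and background music.
; On overlap it calls Use on its SwitchActors, then spawns and enables each ActorSpawnArea.
; Sequence playback runs through BP_GI_Main, with music either handed to the sequence to play afterwards or set right away.
; With ExecuteOnce set, the trigger destroys itself after firing.
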(event Collision|EventActorBeginOverlap
  (params (OtherActor :type Actor%20Object%20Reference))
  (bind _backgroundmusictobeplayed (Variables|Audio|GetBackGroundMusicToBePlayed))
  (bind _sequencetobeplayed (Variables|Sequence|GetSequenceToBePlayed))
  (bind _sequencetobeplayed_2 (Variables|Sequence|GetSequenceToBePlayed))
  ;[1 1 1] Save GameInstance Ref.
  (bind _asbp_gi_main (Utilities|Casting|CastToBP_GI_Main (Game|GetGameInstance)))
  (Variables|General|SetGameInstance _asbp_gi_main)
  ;[1 1 1] Start the use Function of the SwitchActors
  (for _array_element (Variables|Spawn|GetSwitchActors)
    (Utilities|IsValid _array_element
      (:Is%20Valid
        (Default|Use _array_element))))
  ;[1 1 1] Start the SpawnFunction of each SpawnAreas.
  (for _array_element_2 (Variables|Spawn|GetActorSpawnArea)
    (Utilities|IsValid _array_element_2
      (:Is%20Valid
        (Default|Spawn _array_element_2)
        (Variables|/Game/Blueprints/Objects/BP_TB_ActorSpawnArea.BP_TB_ActorSpawnArea_C|SetEnabled? _array_element_2 true))))
  ;[1 1 1] Check Audio Options.
  (if (Variables|Audio|GetPlayBackGroundMusicAfterSequence)
    ;[1 1 1] Sequence Management with Audio Start.
    (Utilities|IsValid _sequencetobeplayed_2
      (:Is%20Valid
        (Default|RunSequence (Variables|General|GetGameInstance) _sequencetobeplayed_2 (Variables|Sequence|GetHidePlayer?) (Variables|Sequence|GetCameraBlendSpeed) (Variables|Sequence|GetDisableAi?) (Variables|Sequence|GetSkipCameraBlendSpeed) (Variables|Audio|GetBackGroundMusicToBePlayed)))
      (:Is%20Not%20Valid
        _))
    (else
      ;[1 1 1] Sequence Management without Audio Start.
      (Utilities|IsValid _sequencetobeplayed
        (:Is%20Valid
          (Default|RunSequence (Variables|General|GetGameInstance) _sequencetobeplayed (Variables|Sequence|GetHidePlayer?) (Variables|Sequence|GetCameraBlendSpeed) (Variables|Sequence|GetDisableAi?) (Variables|Sequence|GetSkipCameraBlendSpeed)))
        (:Is%20Not%20Valid
          _))
      ;[1 1 1] Play BackGroundMusic
      (Utilities|IsValid _backgroundmusictobeplayed
        (:Is%20Valid
          (Default|SetBackGroundMusic (Variables|General|GetGameInstance) _backgroundmusictobeplayed))
        (:Is%20Not%20Valid
          _))))
  ;[1 1 1] If only execute once, destroy the Actor.
  (if (Variables|General|GetExecuteOnce?)
    (Actor|DestroyActor)))

(fn ConstructionScript)