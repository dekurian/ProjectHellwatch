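; BP_AC_Switch is a switch actor that triggers a linked object when another actor overlaps it.
; Overlap calls Use on a valid SwitchObject, then casts the game instance to BP_GI_Main as a gate.
; If that cast succeeds, it also spawns a BP_CH_BasicAI pawn slightly offset from the player character's mesh.
; The construction script applies the configurable SwitchMesh to the Switch component.
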(event EventBeginPlay)

(event Collision|EventActorBeginOverlap
  (params (OtherActor :type Actor%20Object%20Reference))
  (Utilities|IsValid (Variables|Default|GetSwitchObject)
    (:Is%20Valid
      (Default|Use (Variables|Default|GetSwitchObject))
      (Utilities|Casting|CastToBP_GI_Main (Game|GetGameInstance))
      (AI|SpawnAIFromClass "/Game/Blueprints/AI/BP_CH_BasicAI.BP_CH_BasicAI_C" 0 (+ (Transformation|GetWorldLocation (Variables|/Script/Engine.Character|GetMesh (Game|GetPlayerCharacter 0))) "10.000000, 0, 0") "0, 0, 0" false))))

(event EventTick
  (params (DeltaSeconds :type Float%20%28single-precision%29)))

(fn ConstructionScript
  (Components|StaticMesh|SetStaticMesh (Variables|Default|GetSwitch) (Variables|Default|GetSwitchMesh)))