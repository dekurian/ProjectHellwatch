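; Box-volume spawn area that populates itself with AI or other actors, then uses its linked switch actors and destroys itself once no tracked AI remain.
; Spawn places predefined spawn-point actors, then calls SpawnAmount for random types at random box points line-traced downward.
; While enabled, Tick prunes dead BP_CH_BasicAI from the living list and can optionally top up random AI to keep numbers constant.
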(event EventTick
  (params (DeltaSeconds :type Float%20%28single-precision%29))
  (bind _livingaiactors (Variables|Spawn|GetLivingAIActors))
  (bind _livingaiactors_2 (Variables|Spawn|GetLivingAIActors))
  (bind _spawnrandomamount (Variables|Spawn|GetSpawnRandomAmount))
  (bind _predefinedspawnpoints (Variables|Spawn|GetPredefinedSpawnPoints))
  (bind _returnvalue (Utilities|Array|Length _livingaiactors_2))
  (bind _returnvalue_2 (Utilities|Array|Length _predefinedspawnpoints))
  (bind _returnvalue_3 (- _returnvalue _returnvalue_2))
  (bind _returnvalue_4 (- _spawnrandomamount _returnvalue_3))
  ;[1 1 1] Only execute Function if enabled.
  (if (Variables|General|GetEnabled?)
    (Utilities|FlowControl|Sequence
      (:then_0
        ;[1 1 1] Loop through each actor.
        (if (> (Utilities|Array|Length _livingaiactors) 0)
          (for _array_element _livingaiactors
            ;[1 1 1] Remove Actor from the List, if dead.
            (bind _asbp_ch_basic_ai (Utilities|Casting|CastToBP_CH_BasicAI _array_element))
            (if (Variables|/Game/Blueprints/AI/BP_CH_BasicAI.BP_CH_BasicAI_C|GetIsDead? _asbp_ch_basic_ai)
              (Utilities|Array|RemoveItem (Variables|Spawn|GetLivingAIActors) _array_element)))
          (else
            ;[1 1 1] Switch Actor Handling
            (for _array_element_2 (Variables|Switch|GetSwitchActors)
              (Utilities|IsValid _array_element_2
                (:Is%20Valid
                  (Default|Use _array_element_2))))
            ;[1 1 1] Destroy the Actor.
            (Actor|DestroyActor))))
      (:then_1
        ;[1 1 1] Always respawn Actors until we have the max amount of Actors.
        (if (Variables|Spawn|GetAlwaysKeepAmountOfAI)
          (if (Variables|Spawn|GetIsRandomActorAI?)
            (if (> _returnvalue_4 0)
              (CallFunction|SpawnAmount _returnvalue_4))))))))

(event EventBeginPlay
  ;[1 1 1] Save GameInstance Ref.
  (bind _asbp_gi_main (Utilities|Casting|CastToBP_GI_Main (Game|GetGameInstance)))
  (Variables|General|SetGameInstance _asbp_gi_main))

(fn ConstructionScript)

(fn Spawn
  (bind _spawnrandomamount (Variables|Spawn|GetSpawnRandomAmount))
  (for _array_element (Variables|Spawn|GetPredefinedSpawnPoints)
    ;[1 1 1] Spawn the predefined List.
    (if (Variables|/Game/Blueprints/Objects/BP_AC_SpawnPoint.BP_AC_SpawnPoint_C|GetIsAI? _array_element)
      (bind _aspawn (Utilities|Casting|CastToPawnClass (Variables|/Game/Blueprints/Objects/BP_AC_SpawnPoint.BP_AC_SpawnPoint_C|GetActorType _array_element)))
      (bind _returnvalue (AI|SpawnAIFromClass _aspawn 0 (.location (Transformation|GetActorTransform _array_element)) (.rotation (Transformation|GetActorTransform _array_element)) false))
      (Utilities|Array|Add (Variables|Spawn|GetLivingAIActors) _returnvalue)
      (else
        (Game|SpawnActorfromClass (Variables|/Game/Blueprints/Objects/BP_AC_SpawnPoint.BP_AC_SpawnPoint_C|GetActorType _array_element) (Math|Transform|MakeTransform (.location (Transformation|GetActorTransform _array_element)) (.rotation (Transformation|GetActorTransform _array_element)) (.scale (Transformation|GetActorTransform _array_element))) "AdjustIfPossibleButAlwaysSpawn" 0 0))))
  ;[1 1 1] Spawn the amount of random Actor.
  (if (> _spawnrandomamount 0)
    (CallFunction|SpawnAmount _spawnrandomamount)))

(fn SpawnAmount
  (params (Amount :type Integer))
  (bind _returnvalue (Math|Random|RandomFloatinRange 0.0 3.6e+02))
  (bind _actortypes (Variables|Spawn|GetActorTypes))
  (bind _returnvalue_2 (Utilities|Array|LastIndex _actortypes))
  (bind _returnvalue_3 (Math|Rotator|MakeRotator 0.0 0.0 _returnvalue))
  (bind _returnvalue_4 (Math|Random|RandomIntegerinRange 0 _returnvalue_2))
  (bind _item (Utilities|Array|Get(acopy) _actortypes _returnvalue_4))
  ;[1 1 1] Spawn Random Actors.
  (for _index (range 1 Amount)
    (bind _asbox_collision (Utilities|Casting|CastToBoxComponent (Variables|Default|GetCollisionComponent)))
    (if (Utilities|Array|IsValidIndex _actortypes _returnvalue_4)
      (bind _outhit (Collision|LineTraceByChannel (Math|Random|RandomPointinBoundingBox (Transformation|GetActorLocation self) (Math|Vector|MakeVector (.x (Variables|/Script/Engine.BoxComponent|GetBoxExtent _asbox_collision)) (.y (Variables|/Script/Engine.BoxComponent|GetBoxExtent _asbox_collision)) (.z (Variables|/Script/Engine.BoxComponent|GetBoxExtent _asbox_collision)))) (- (Math|Random|RandomPointinBoundingBox (Transformation|GetActorLocation self) (Math|Vector|MakeVector (.x (Variables|/Script/Engine.BoxComponent|GetBoxExtent _asbox_collision)) (.y (Variables|/Script/Engine.BoxComponent|GetBoxExtent _asbox_collision)) (.z (Variables|/Script/Engine.BoxComponent|GetBoxExtent _asbox_collision)))) "0, 0,99999.000000") "TraceTypeQuery1" false 0 "None"))
      (if (Variables|Spawn|GetIsRandomActorAI?)
        (bind _aspawn (Utilities|Casting|CastToPawnClass _item))
        (bind _returnvalue_5 (AI|SpawnAIFromClass _aspawn 0 (.Location (Collision|BreakHitResult _outhit)) _returnvalue_3 false))
        (Utilities|Array|Add (Variables|Spawn|GetLivingAIActors) _returnvalue_5)
        (else
          (Game|SpawnActorfromClass _item (Math|Transform|MakeTransform (.Location (Collision|BreakHitResult _outhit)) _returnvalue_3 "1.000000,1.000000,1.000000") "AdjustIfPossibleButAlwaysSpawn" 0 0))))))