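; BP_TB_Objective is a one-time trigger that completes a task when something overlaps its collision component.
; On overlap it tells BP_GI_Main to complete TaskToComplete, records its EventSwitchID in the save game, then destroys itself.
; On BeginPlay it destroys itself if that switch is already saved.
; The construction script derives the switch ID from the actor's display name.
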(event OnComponentBeginOverlap(CollisionComponent)
  (params (OverlappedComponent :type Primitive%20Component%20Object%20Reference) (OtherActor :type Actor%20Object%20Reference) (OtherComp :type Primitive%20Component%20Object%20Reference) (OtherBodyIndex :type Integer) (bFromSweep :type Boolean) (SweepResult :type Hit%20Result%20Structure%20%28by%20ref%29))
  ;[1 1 1] Complete the given Task.
  (Default|CompleteTask (Variables|Default|GetGameInstance) (Variables|Mission|GetTaskToComplete))
  ;[1 1 1] Add the Event Switch.
  (Default|AddEventSwitch (Default|GetSaveGame (Variables|Default|GetGameInstance)) (Variables|Mission|GetEventSwitch%20ID))
  (Actor|DestroyActor))

(event EventBeginPlay
  ;[1 1 1] Get tthe GameInstance.
  (bind _asbp_gi_main (Utilities|Casting|CastToBP_GI_Main (Game|GetGameInstance)))
  (Variables|Default|SetGameInstance _asbp_gi_main)
  ;[1 1 1] Check if the Event has been called already.
  (bind _exists (Default|CheckEventSwitch (Default|GetSaveGame (Variables|Default|GetGameInstance)) (Variables|Mission|GetEventSwitch%20ID)))
  (if _exists
    (Actor|DestroyActor)))

(event Collision|EventActorBeginOverlap
  (params (OtherActor :type Actor%20Object%20Reference)))

(event EventTick
  (params (DeltaSeconds :type Float%20%28single-precision%29)))

(fn ConstructionScript
  ;[1 1 1] Set the Name of the Object.
  (Variables|Mission|SetEventSwitch%20ID (Utilities|GetDisplayName self)))