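; BP_AC_SA_FightBarrier is a toggleable barrier object, named for fights, built around a Cube component.
; On BeginPlay it hides the cube and turns off its collision, so the barrier starts inactive.
; Each Use event flips the Enabled flag, either showing the cube with query and physics collision or hiding it with no collision.
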(event EventBeginPlay
  (bind _cube (Variables|Default|GetCube))
  (Development|SetHiddeninGame _cube true false)
  (Collision|SetCollisionEnabled _cube "NoCollision"))

(event EventUse
  (bind _cube (Variables|Default|GetCube))
  (bind _cube_2 (Variables|Default|GetCube))
  (if (Variables|Default|GetEnabled?)
    (Variables|Default|SetEnabled? false)
    (Development|SetHiddeninGame _cube_2 true false)
    (Collision|SetCollisionEnabled _cube_2 "NoCollision")
    (else
      (Variables|Default|SetEnabled? true)
      (Development|SetHiddeninGame _cube false false)
      (Collision|SetCollisionEnabled _cube "QueryAndPhysics"))))

(fn ConstructionScript
  (|CallParentFunction))