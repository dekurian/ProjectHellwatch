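; Cutscene handler that plays a level sequence when an actor overlap fires, locking player movement and turning in cinematic mode.
; It disables movement on every actor of a class during playback, then restores walking when a timer matched to the sequence length calls EndSequence.
; SpaceBar skips to the end, and Enter toggles pause for the sequence, timer and game together.
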(event OnActorBeginOverlap()
  (params (OverlappedActor :type Actor%20Object%20Reference) (OtherActor :type Actor%20Object%20Reference))
  (bind _sequenceplayer (Variables|/Script/LevelSequence.LevelSequenceActor|GetSequencePlayer "Literal"))
  (Components|Timeline|SetPlaybackPosition _sequenceplayer 0.0)
  (Class|LevelScriptActor|SetCinematicMode true false false true true)
  (Actor|GetAllActorsOfClass 0)
  (for _array_element 0
    (Pawn|Components|CharacterMovement|DisableMovement (Variables|/Script/Engine.Character|GetCharacterMovement _array_element)))
  (Audio|Components|Audio|Play _sequenceplayer)
  (bind _returnvalue (Utilities|Time|SetTimerbyEvent (delegate Custom|EndSequence) (Class|LevelSequencePlayer|GetLength _sequenceplayer)))
  (Variables|Default|SetHandleSequenceTimer _returnvalue))

(event Custom|EndSequence
  (Class|LevelScriptActor|SetCinematicMode false false false true true)
  (Actor|GetAllActorsOfClass 0)
  (for _array_element 0
    (Pawn|Components|CharacterMovement|SetMovementMode (Variables|/Script/Engine.Character|GetCharacterMovement _array_element) "MOVE_Walking" 0)))

(event Input|KeyboardEvents|SpaceBar
  (params (Key :type Key%20Structure :default "AnyKey"))
  (bind _sequenceplayer (Variables|/Script/LevelSequence.LevelSequenceActor|GetSequencePlayer "Literal"))
  (:Pressed
    (Utilities|Time|ClearandInvalidateTimerbyHandle (Variables|Default|GetHandleSequenceTimer))
    (Components|Timeline|SetPlaybackPosition _sequenceplayer (Class|LevelSequencePlayer|GetLength _sequenceplayer))
    (CallFunction|EndSequence)))

(event Input|KeyboardEvents|Enter
  (params (Key :type Key%20Structure :default "AnyKey"))
  (bind _handlesequencetimer (Variables|Default|GetHandleSequenceTimer))
  (bind _sequenceplayer (Variables|/Script/LevelSequence.LevelSequenceActor|GetSequencePlayer "Literal"))
  (:Pressed
    (if (Audio|Components|Audio|IsPlaying _sequenceplayer)
      (Utilities|Time|PauseTimerbyHandle _handlesequencetimer)
      (Sequencer|Player|Pause _sequenceplayer)
      (Game|SetGamePaused true)
      (else
        (Utilities|Time|UnpauseTimerbyHandle _handlesequencetimer)
        (Audio|Components|Audio|Play _sequenceplayer)
        (Game|SetGamePaused false)))))

(fn ConstructionScript)