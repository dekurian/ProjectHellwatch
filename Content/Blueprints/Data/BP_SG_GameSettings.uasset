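; BP_SG_GameSettings is a settings data object, apparently a SaveGame, holding player options for audio, subtitles, language and graphics.
; Simple getter and setter pairs expose volume levels, subtitle and language choices, post-process toggles and the anti-aliasing method.
; It also holds save slot records, with read-only functions to fetch a slot by index, report the last active one and check whether that slot is valid and in use.
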(fn GetMusicVolume
  (return (Variables|AudioSettings|GetVolumeMusic)))

(fn GetDialogueVolume
  (return (Variables|AudioSettings|GetVolumeDialogue)))

(fn GetSFXVolume
  (return (Variables|AudioSettings|GetVolumeSFX)))

(fn GetSubtitles
  (return (Variables|AudioSettings|GetSubtitles)))

(fn GetLanguageText
  (return (Variables|AudioSettings|GetLanguageText)))

(fn SetMusicVolume
  (params (MusicVolume :type Float%20%28single-precision%29))
  (Variables|AudioSettings|SetVolumeMusic MusicVolume))

(fn SetDialogueVolume
  (params (DialogueVolume :type Float%20%28single-precision%29))
  (Variables|AudioSettings|SetVolumeDialogue DialogueVolume))

(fn SetSFXVolume
  (params (SFXVolume :type Float%20%28single-precision%29))
  (Variables|AudioSettings|SetVolumeSFX SFXVolume))

(fn SetSubtitles
  (params (Subtitles :type Boolean))
  (Variables|AudioSettings|SetSubtitles Subtitles))

(fn SetLanguageText
  (params (Language%20Text :type Integer))
  (Variables|AudioSettings|SetLanguageText Language%20Text))

(fn GetPPMotionBlur
  (return (Variables|GraphicsSettings|GetPP_MotionBlur)))

(fn SetPPMotionBlur
  (params (Enabled? :type Boolean))
  (Variables|GraphicsSettings|SetPP_MotionBlur Enabled?))

(fn GetPPSSAO
  (return (Variables|GraphicsSettings|GetPP_SSAO)))

(fn SetPPSSAO
  (params (Enabled? :type Boolean))
  (Variables|GraphicsSettings|SetPP_SSAO Enabled?))

(fn GetPPBloom
  (return (Variables|GraphicsSettings|GetPP_Bloom)))

(fn SetPPBloom
  (params (Enabled? :type Boolean))
  (Variables|GraphicsSettings|SetPP_Bloom Enabled?))

(fn GetPPAutoExposure
  (return (Variables|GraphicsSettings|GetPP_AutoExposure)))

(fn SetPPAutoExposure
  (params (Enabled? :type Boolean))
  (Variables|GraphicsSettings|SetPP_AutoExposure Enabled?))

(fn GetPPLensflares
  (return (Variables|GraphicsSettings|GetPP_Lensflares)))

(fn SetPPLensflares
  (params (Enabled? :type Boolean))
  (Variables|GraphicsSettings|SetPP_Lensflares Enabled?))

(fn GetAAMethod
  (return (Variables|GraphicsSettings|GetAAMethod)))

(fn SetAAMethod
  (params (AAMethod :type Integer))
  (Variables|GraphicsSettings|SetAAMethod AAMethod))

(fn GetSaveSlotbyIndex
  (params (SaveSlot :type Integer))
  (if (Utilities|Array|IsValidIndex (Variables|SaveGames|GetSaveSlots) SaveSlot)
    (return (Utilities|Array|Get(acopy) (Variables|SaveGames|GetSaveSlots) SaveSlot))
    (else
      (return ""))))

(fn IsSaveGameAvailable
  ;[1 1 1] Check if there's a last active SaveSlot and return if it's valid
  (if (Utilities|Array|IsValidIndex (Variables|SaveGames|GetSaveSlots) (Variables|SaveGames|GetLastActiveSaveSlot))
    (return (.isinuse (Utilities|Array|Get(acopy) (Variables|SaveGames|GetSaveSlots) (Variables|SaveGames|GetLastActiveSaveSlot))))
    (else
      (return false))))

(fn GetLastActiveSaveSlot
  (return (Variables|SaveGames|GetLastActiveSaveSlot)))