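; Player character Blueprint handling walk and look input with optional vertical inversion, a Shift slow walk, and a Jump key that skips any playing sequence through the game mode.
; When foot IK is enabled, Tick line-traces below each foot socket and interpolates scale-corrected offsets, using a trace distance derived at construction.
; It also resizes the capsule radius from a sphere trace around the character, resetting it when IK is off.
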(event EventTick
  (params (DeltaSeconds :type Float%20%28single-precision%29))
  (Utilities|FlowControl|Sequence
    (:then_1
      ;[1 1 1] IK Foot Tracing
      (if (Variables|Default|GetIsIKFootEnabled?)
        (Utilities|FlowControl|Sequence
          (:then_0
            (bind _ik_offset (CallFunction|IkFootTrace (Variables|AnimationHandler|IKFeet|GetIKTraceDistance) (Variables|AnimationHandler|IKFeet|GetRightFootSocket))) ; IK for right Foot
            (if (< (Math|Interpolation|FInterpTo (Variables|AnimationHandler|IKFeet|GetIK%20OffsetRightFoot) _ik_offset (Utilities|Time|GetWorldDeltaSeconds) (Variables|AnimationHandler|IKFeet|GetIKInterpSpeed)) 4e+01)
              (Variables|AnimationHandler|IKFeet|SetIK%20OffsetRightFoot (Math|Interpolation|FInterpTo (Variables|AnimationHandler|IKFeet|GetIK%20OffsetRightFoot) _ik_offset (Utilities|Time|GetWorldDeltaSeconds) (Variables|AnimationHandler|IKFeet|GetIKInterpSpeed)))
              (bind _ik_offset_2 (CallFunction|IkFootTrace (Variables|AnimationHandler|IKFeet|GetIKTraceDistance) (Variables|AnimationHandler|IKFeet|GetLeftFootSocket))) ; IK for left Foot
              (if (< (Math|Interpolation|FInterpTo (Variables|AnimationHandler|IKFeet|GetIK%20OffsetLeftFoot) _ik_offset_2 (Utilities|Time|GetWorldDeltaSeconds) (Variables|AnimationHandler|IKFeet|GetIKInterpSpeed)) 4e+01)
                (Variables|AnimationHandler|IKFeet|SetIK%20OffsetLeftFoot (Math|Interpolation|FInterpTo (Variables|AnimationHandler|IKFeet|GetIK%20OffsetLeftFoot) _ik_offset_2 (Utilities|Time|GetWorldDeltaSeconds) (Variables|AnimationHandler|IKFeet|GetIKInterpSpeed))))))
          (:then_1
            (|AdjustCapsuleComponent)))
        (else
          (Components|Capsule|SetCapsuleRadius (Variables|Collision|GetCapsuleComponent) 34.0 true))))))

(event Input|ActionEvents|InputActionJump
  (params (Key :type Key%20Structure :default "AnyKey"))
  ;[1 1 1] Space Behaviour
  (:Pressed
    (bind _asbp_gm_main (Utilities|Casting|CastToBP_GM_Main (Game|GetGameMode)))
    (bind _asbp_gs_main (Utilities|Casting|CastToBP_GS_Main (Game|GetGameState)))
    (if (Variables|/Game/Blueprints/Framework/BP_GS_Main.BP_GS_Main_C|GetIsInSequence _asbp_gs_main)
      (Default|SkipSequence _asbp_gm_main (Variables|/Game/Blueprints/Framework/BP_GS_Main.BP_GS_Main_C|GetCurrentSequence _asbp_gs_main) self 0.0)
      (else
        (Character|Jump)))))

(event Input|AxisEvents|InputAxisMoveForward
  (params (AxisValue :type Float%20%28single-precision%29))
  ;[1 1 1] Movement Keyboard
  (Pawn|Input|AddMovementInput (Math|Vector|GetForwardVector (Math|Rotator|MakeRotator 0.0 0.0 (.Yaw (Math|Rotator|BreakRotator (Pawn|GetControlRotation :!class /Script/Engine.Pawn))))) AxisValue false))

(event Input|AxisEvents|InputAxisVerticalTurn
  (params (AxisValue :type Float%20%28single-precision%29))
  (bind _verticalsensivityforce (Variables|ControlSettings|GetVerticalSensivityForce))
  (bind _returnvalue (* AxisValue _verticalsensivityforce))
  ;[1 1 1] Mouse Movement
  (if (Variables|ControlSettings|GetInvert%20Vertically)
    (Pawn|Input|AddControllerPitchInput (* _returnvalue -1.0))
    (else
      (Pawn|Input|AddControllerPitchInput _returnvalue))))

(event Input|AxisEvents|InputAxisHorizontalForce
  (params (AxisValue :type Float%20%28single-precision%29))
  ;[1 1 1] Controller Input
  (Pawn|Input|AddControllerYawInput (* AxisValue (Utilities|Time|GetWorldDeltaSeconds) (Variables|ControlSettings|GetHorizontalForce))))

(event Input|AxisEvents|InputAxisVerticalForce
  (params (AxisValue :type Float%20%28single-precision%29))
  (bind _returnvalue (Utilities|Time|GetWorldDeltaSeconds))
  (bind _verticalforce (Variables|ControlSettings|GetVerticalForce))
  (bind _returnvalue_2 (* AxisValue _returnvalue _verticalforce))
  ;[1 1 1] Controller Input
  (if (Variables|ControlSettings|GetInvert%20Vertically)
    (Pawn|Input|AddControllerPitchInput (* _returnvalue_2 -1.0))
    (else
      (Pawn|Input|AddControllerPitchInput _returnvalue_2))))

(event Input|AxisEvents|InputAxisMoveRight
  (params (AxisValue :type Float%20%28single-precision%29))
  ;[1 1 1] Movement Keyboard
  (Pawn|Input|AddMovementInput (Math|Vector|GetRightVector (Math|Rotator|MakeRotator 0.0 0.0 (.Yaw (Math|Rotator|BreakRotator (Pawn|GetControlRotation :!class /Script/Engine.Pawn))))) AxisValue false))

(event Input|AxisEvents|InputAxisHorizontalTurn
  (params (AxisValue :type Float%20%28single-precision%29))
  ;[1 1 1] Mouse Movement
  (Pawn|Input|AddControllerYawInput (* AxisValue (Variables|ControlSettings|GetHorizontalSensivityForce))))

(event Input|KeyboardEvents|LeftShift
  (params (Key :type Key%20Structure :default "AnyKey"))
  (bind _charactermovement (Variables|Character|GetCharacterMovement))
  ;[1 1 1] Movement Keyboard
  (:Pressed
    (Variables|/Script/Engine.CharacterMovementComponent|SetMaxWalkSpeed _charactermovement 1.5e+02))
  (:Released
    (Variables|/Script/Engine.CharacterMovementComponent|SetMaxWalkSpeed _charactermovement (Variables|ControlSettings|GetInitWalkSpeed))))

(fn ConstructionScript
  ;[1 1 1] Save Character Attributes
  (Variables|ControlSettings|SetInitWalkSpeed (Variables|/Script/Engine.CharacterMovementComponent|GetMaxWalkSpeed (Variables|Character|GetCharacterMovement)))
  ;[1 1 1] Set IK Trace Distance Variables
  (Variables|AnimationHandler|IKFeet|SetScale (.Z (Math|Vector|BreakVector (.Scale (Math|Transform|BreakTransform (Transformation|GetActorTransform))))))
  (Variables|AnimationHandler|IKFeet|SetIKTraceDistance (* (Variables|/Script/Engine.CapsuleComponent|GetCapsuleHalfHeight (Variables|Collision|GetCapsuleComponent)) (Variables|AnimationHandler|IKFeet|GetScale))))

(fn IkFootTrace
  (params (TraceDistance :type Float%20%28single-precision%29) (Socket :type Name))
  (bind _returnvalue (Transformation|GetActorLocation))
  (bind _mesh (Variables|Character|GetMesh))
  (bind _returnvalue_2 (Transformation|GetSocketLocation _mesh Socket))
  (bind _z (Math|Vector|BreakVector _returnvalue))
  (bind (_x _y) (Math|Vector|BreakVector _returnvalue_2))
  (bind _returnvalue_3 (- _z TraceDistance))
  (bind _returnvalue_4 (Math|Vector|MakeVector _x _y _returnvalue_3))
  (bind (_outhit _returnvalue_5) (Collision|LineTraceByChannel (Math|Vector|MakeVector _x _y _z) _returnvalue_4 "TraceTypeQuery1" false (Utilities|Array|MakeArray (Components|GetOwner (Variables|Collision|GetCapsuleComponent))) "None"))
  (return (Math|Float|SelectFloat (/ (Math|Vector|VectorLength (- (.Location (Collision|BreakHitResult _outhit)) _returnvalue_4)) (Variables|AnimationHandler|IKFeet|GetScale)) 0.0 _returnvalue_5)))