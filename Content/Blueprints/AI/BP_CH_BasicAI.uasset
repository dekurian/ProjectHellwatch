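; Basic AI character that chases pawns it sees and dies on contact with the main character.
; On BeginPlay it registers itself in BP_GM_Main's active AI list.
; PawnSensing drives a simple move-to-actor chase unless it is dead or in a nav link proxy event.
; A hit involving the main character removes it from the list, enables physics on mesh and capsule, and marks it dead.
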(event OnSeePawn(PawnSensing)
  (params (Pawn :type Pawn%20Object%20Reference))
  ;[1 1 1] If the AI sees the Player, the AI should run to him.
  (if (not (Variables|Default|GetIsDead?))
    (if (not (Variables|Default|GetIsInNavLinkProxyEvent?))
      (AI|Navigation|SimpleMovetoActor (Pawn|GetController self) Pawn))))

(event EventBeginPlay
  ;[1 1 1] On Level Begin they need to be added to the current GameMode, since we want to be able to reference them.
  (bind _asbp_gm_main (Utilities|Casting|CastToBP_GM_Main (Game|GetGameMode)))
  (Variables|Default|SetGameMode _asbp_gm_main)
  (Utilities|Array|Add (Variables|/Game/Blueprints/Framework/BP_GM_Main.BP_GM_Main_C|GetActiveAIActors _asbp_gm_main) self))

(event Collision|EventHit
  (params (MyComp :type Primitive%20Component%20Object%20Reference) (Other :type Actor%20Object%20Reference) (OtherComp :type Primitive%20Component%20Object%20Reference) (bSelfMoved :type Boolean) (HitLocation :type Vector :default "0, 0, 0") (HitNormal :type Vector :default "0, 0, 0") (NormalImpulse :type Vector :default "0, 0, 0") (Hit :type Hit%20Result%20Structure%20%28by%20ref%29))
  (bind _self self)
  (bind _gamemode (Variables|Default|GetGameMode))
  (bind _activeaiactors (Variables|/Game/Blueprints/Framework/BP_GM_Main.BP_GM_Main_C|GetActiveAIActors _gamemode))
  ;[1 1 1] If the AI dies, remove it from the Active List.
  (if (== (.HitActor (Collision|BreakHitResult Hit)) (Variables|/Game/Blueprints/Framework/BP_GM_Main.BP_GM_Main_C|GetMainCharacter (Variables|Default|GetGameMode)))
    (if (>= (Utilities|Array|FindItem _activeaiactors _self) 0)
      (Utilities|Array|RemoveItem _activeaiactors _self)
      (Physics|SetSimulatePhysics (Variables|Character|GetMesh) true)
      (Physics|SetSimulatePhysics (Variables|Collision|GetCapsuleComponent) true)
      (Variables|Default|SetIsDead? true))))

(fn ConstructionScript)