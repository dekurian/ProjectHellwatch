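; Main menu game mode that holds menu state, difficulty and save slot selection, and starts, loads or continues a game.
; SetMainMenuState fires a state-changed event with old and new states before storing the new one.
; New Game has BP_GI_Main initialize mission 1 and create a save from the selected slot and difficulty.
; Load and Continue share one path using the current save's mission; all open MAP_Main_00.
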(event EventBeginPlay
  (bind _asbp_gi_main (Utilities|Casting|CastToBP_GI_Main (Game|GetGameInstance)))
  (Variables|Default|SetGameInstance _asbp_gi_main))

(fn ConstructionScript)

(fn GetMainMenuState
  ;[1 1 1] Get current Main-Menu-State
  (return (Variables|Default|GetMainMenuState)))

(fn SetMainMenuState
  (params (newMainMenuState :type BPE_MainMenuState%20Enum))
  ;[1 1 1] Set current Main-Menu-State and Call State-Changed-Event
  (Default|CallOnMenuStateChanged (Variables|Default|GetMainMenuState) newMainMenuState)
  (Variables|Default|SetMainMenuState newMainMenuState))

(fn SetSelectedDifficulty
  (params (SelectedDifficulty :type BPE_GameDifficulty%20Enum))
  (Variables|Default|SetSelectedDifficulty SelectedDifficulty))

(fn GetSelectedDifficulty
  (return (Variables|Default|GetSelectedDifficulty)))

(fn InitNewGame
  (Default|LoadMission (Variables|Default|GetGameInstance) 1 true)
  (Default|CreateNewSaveGame (Variables|Default|GetGameInstance) (Variables|Default|GetSelectedSaveSlot) (Variables|Default|GetSelectedDifficulty))
  (Game|OpenLevel(byName) "MAP_Main_00"))

(fn SetSelectedSaveSlot
  (params (SelectedSlot :type Integer))
  (Variables|Default|SetSelectedSaveSlot SelectedSlot))

(fn GetSelectedSaveSlot
  (return (Variables|Default|GetSelectedSaveSlot)))

(fn InitLoadGame
  (Default|LoadMission (Variables|Default|GetGameInstance) (Default|GetCurrentMissionID (Default|GetSaveGame (Variables|Default|GetGameInstance))) false)
  (Game|OpenLevel(byName) "MAP_Main_00"))

(fn InitContinue
  (CallFunction|InitLoadGame))

(fn SetSaveSlotSelectionMode
  (params (NewParam :type BPE_SaveSelectionMode%20Enum))
  (Variables|Default|SetSaveSlotSelectionMode NewParam))

(fn GetSaveSlotSelectionMode
  (return (Variables|Default|GetSaveSlotSelectionMode)))