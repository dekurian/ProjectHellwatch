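; Main game instance that provides cutscene control, pausing, settings persistence and system message boxes across the game.
; Sequences play in cinematic mode with optional AI movement freeze, using a length-based timer that pauses with playback or clears on skip.
; Ending blends the camera back to the main character, while ReinitGameplay restores controls and AI walking.
; Settings load on Init from a SaveGame slot, created if missing, with failed saves reported in a reused message widget.
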(event EventInit
  (GameSettings|LoadGameSettings))

(fn RunSequence
  (params (SequenceToBePlayed :type Level%20Sequence%20Actor%20Object%20Reference) (HidePlayerDuringSequence? :type Boolean) (CameraBlendSpeed :type Float%20%28single-precision%29) (DisableAi? :type Boolean))
  ;[1 1 1] Save Parameters
  (LocalVariables|SetlocalSequence SequenceToBePlayed)
  (LocalVariables|SetlocalHidePlayer HidePlayerDuringSequence?)
  (LocalVariables|SetLocalCameraBlendSpeed CameraBlendSpeed)
  (LocalVariables|SetlocalDisableAi DisableAi?)
  ;[1 1 1] First get the GameMode since we need it here.
  (bind _asbp_gm_main (Utilities|Casting|CastToBP_GM_Main (Game|GetGameMode)))
  (LocalVariables|SetlocalGameMode _asbp_gm_main)
  ;[1 1 1] Init the Sequence and set the Position to 0, so we can trigger the Sequence again and again.
  (CallFunction|SetSequenceInfo true (LocalVariables|GetlocalSequence) (LocalVariables|GetLocalCameraBlendSpeed))
  (Components|Timeline|SetPlaybackPosition (Variables|/Script/LevelSequence.LevelSequenceActor|GetSequencePlayer (LocalVariables|GetlocalSequence)) 0.0)
  (Class|PlayerController|SetCinematicMode (Game|GetPlayerController 0) true (LocalVariables|GetlocalHidePlayer) true true true)
  ;[1 1 1] Disable Movement of all AI
  (if (LocalVariables|GetlocalDisableAi)
    (for _array_element (Variables|/Game/Blueprints/Framework/BP_GM_Main.BP_GM_Main_C|GetActiveAIActors (LocalVariables|GetlocalGameMode))
      (Pawn|Components|CharacterMovement|DisableMovement (Variables|/Script/Engine.Character|GetCharacterMovement _array_element))))
  ;[1 1 1] Play the Actual Scene and specify the EndEvent.
  (Audio|Components|Audio|Play (Variables|/Script/LevelSequence.LevelSequenceActor|GetSequencePlayer (LocalVariables|GetlocalSequence)))
  (bind _returnvalue (Utilities|Time|SetTimerbyEvent (EventDispatchers|CreateEvent :!event EndSequence) (Class|LevelSequencePlayer|GetLength (Variables|/Script/LevelSequence.LevelSequenceActor|GetSequencePlayer (LocalVariables|GetlocalSequence)))))
  (Variables|Sequence|SetHandleSequenceTimer _returnvalue))

(fn EndSequence
  (bind _returnvalue (Game|GetPlayerController 0))
  (bind _sequencecamerablendspeed (Variables|Sequence|GetSequenceCameraBlendSpeed))
  ;[1 1 1] Save reference to the GameMode
  (bind _asbp_gm_main (Utilities|Casting|CastToBP_GM_Main (Game|GetGameMode)))
  (bind _output_get (LocalVariables|SetLocalGameMode _asbp_gm_main))
  ;[1 1 1] End the Sequence
  (bind _asbp_ch_main_character (Utilities|Casting|CastToBP_CH_MainCharacter (Variables|/Game/Blueprints/Framework/BP_GM_Main.BP_GM_Main_C|GetMainCharacter _output_get)))
  (Game|Player|SetViewTargetwithBlend _returnvalue _asbp_ch_main_character _sequencecamerablendspeed "VTBlend_Linear" 0.0 false)
  (Class|PlayerController|SetCinematicMode _returnvalue false false false false false)
  (Utilities|Time|SetTimerbyEvent (EventDispatchers|CreateEvent :!event ReinitGameplay) _sequencecamerablendspeed))

(fn PauseSequence
  (bind _currentsequence (Variables|Sequence|GetCurrentSequence))
  (bind _handlesequencetimer (Variables|Sequence|GetHandleSequenceTimer))
  (bind _sequenceplayer (Variables|/Script/LevelSequence.LevelSequenceActor|GetSequencePlayer _currentsequence))
  ;[1 1 1] We need to know if the sequence is running or not.
  (if (Audio|Components|Audio|IsPlaying _sequenceplayer)
    ;[1 1 1] Pause the Sequence
    (Utilities|Time|PauseTimerbyHandle _handlesequencetimer)
    (Sequencer|Player|Pause _sequenceplayer)
    (Game|SetGamePaused true)
    (else
      ;[1 1 1] Unpause the Sequence.
      (Utilities|Time|UnpauseTimerbyHandle _handlesequencetimer)
      (Audio|Components|Audio|Play _sequenceplayer)
      (Game|SetGamePaused false))))

(fn SkipSequence
  (params (Camera%20Blend%20Speed :type Float%20%28single-precision%29))
  (bind _currentsequence (Variables|Sequence|GetCurrentSequence))
  (bind _sequenceplayer (Variables|/Script/LevelSequence.LevelSequenceActor|GetSequencePlayer _currentsequence))
  ;[1 1 1] Save parameter.
  (LocalVariables|SetLocalCameraBlendSpeed Camera%20Blend%20Speed)
  ;[1 1 1] Set SequenceInfo
  (CallFunction|SetSequenceInfo (Variables|Sequence|GetIsInSequence) (Variables|Sequence|GetCurrentSequence) (LocalVariables|GetLocalCameraBlendSpeed))
  ;[1 1 1] Set the Playback Position to the end of the current Sequence so we skip it and finish the rest.
  (Utilities|Time|ClearandInvalidateTimerbyHandle (Variables|Sequence|GetHandleSequenceTimer))
  (Components|Timeline|SetPlaybackPosition _sequenceplayer (Class|LevelSequencePlayer|GetLength _sequenceplayer))
  (CallFunction|EndSequence))

(fn SetSequenceInfo
  (params (IsInSequence? :type Boolean) (CurrentSequence :type Level%20Sequence%20Actor%20Object%20Reference) (Camera%20Blend%20Speed :type Float%20%28single-precision%29))
  ;[1 1 1] Set relevant information.
  (Variables|Sequence|SetIsInSequence IsInSequence?)
  (Variables|Sequence|SetCurrentSequence CurrentSequence)
  (Variables|Sequence|SetSequenceCameraBlendSpeed Camera%20Blend%20Speed))

(fn ReinitGameplay
  ;[1 1 1] Revoke Cinematic Mode and set Sequence Info
  (Class|PlayerController|SetCinematicMode (Game|GetPlayerController 0) false false true true true)
  (CallFunction|SetSequenceInfo false 0 0.0)
  ;[1 1 1] Get the GameMode
  (bind _asbp_gm_main (Utilities|Casting|CastToBP_GM_Main (Game|GetGameMode)))
  ;[1 1 1] Enable the Movement of the AI again.
  (for _array_element (Variables|/Game/Blueprints/Framework/BP_GM_Main.BP_GM_Main_C|GetActiveAIActors _asbp_gm_main)
    (Pawn|Components|CharacterMovement|SetMovementMode (Variables|/Script/Engine.Character|GetCharacterMovement _array_element) "MOVE_Walking" 0)))

(fn ShowMessagebox
  (params (MessageText :type Text) (MessageTitle :type Text) (MessageType :type BPE_MessageType%20Enum) (MessageIcon :type BPE_MessageIcon%20Enum))
  ;[1 1 1] Create and initialize a new System-Message-Box
  (Utilities|IsValid (Variables|Default|GetSystemMessage)
    (:Is%20Valid
      _)
    (:Is%20Not%20Valid
      (bind _returnvalue (UserInterface|CreateWidget "/Game/UI/UI_SystemMessage_00.UI_SystemMessage_00_C"))
      (Variables|Default|SetSystemMessage _returnvalue)))
  (Default|InitializeMessageBox (Variables|Default|GetSystemMessage) MessageText MessageTitle MessageType MessageIcon)
  (if (UserInterface|Viewport|IsinViewport (Variables|Default|GetSystemMessage))
    _
    (else
      (UserInterface|Viewport|AddtoViewport (Variables|Default|GetSystemMessage) 0)))
  (return (Variables|Default|GetSystemMessage)))

(fn PauseGame
  (if (Variables|Overall|GetIsGamePaused)
    (Game|SetGamePaused false)
    (Variables|Overall|SetIsGamePaused false)
    (else
      (Game|SetGamePaused true)
      (Variables|Overall|SetIsGamePaused true))))

(fn SaveGameSettings
  (Utilities|IsValid (Variables|GameSettings|GetGameSettings)
    (:Is%20Valid
      _)
    (:Is%20Not%20Valid
      (bind _returnvalue (SaveGame|CreateSaveGameObject "/Game/Blueprints/Data/BP_SG_GameSettings.BP_SG_GameSettings_C"))
      (bind _asbp_sg_game_settings (Utilities|Casting|CastToBP_SG_GameSettings _returnvalue))
      (Variables|GameSettings|SetGameSettings _asbp_sg_game_settings)))
  (bind _returnvalue_2 (SaveGame|SaveGametoSlot (Variables|GameSettings|GetGameSettings) (Variables|GameSettings|GetslotGameSettings)))
  (if (not _returnvalue_2)
    (bind _messagebox (CallFunction|ShowMessagebox "There was a problem while saving the Gamesettings. 
Please make sure that there is enough space and that you have the necessary user rights to create a save file." "Save Settings" "NewEnumerator0" "NewEnumerator3"))
    (EventDispatchers|BindEventtoConfirm _messagebox (EventDispatchers|CreateEvent :!event QuitGame))))

(fn LoadGameSettings
  (bind _returnvalue (SaveGame|DoesSaveGameExist (Variables|GameSettings|GetslotGameSettings)))
  (if _returnvalue
    (bind _returnvalue_2 (SaveGame|LoadGamefromSlot (Variables|GameSettings|GetslotGameSettings)))
    (bind _asbp_sg_game_settings (Utilities|Casting|CastToBP_SG_GameSettings _returnvalue_2))
    (Variables|GameSettings|SetGameSettings _asbp_sg_game_settings)
    (else
      (GameSettings|SaveGameSettings))))

(fn QuitGame
  (CallFunction|QuitGame))

(fn GetGameSettings
  (Utilities|IsValid (Variables|GameSettings|GetGameSettings)
    (:Is%20Valid
      (return (Variables|GameSettings|GetGameSettings)))
    (:Is%20Not%20Valid
      (GameSettings|LoadGameSettings)
      (return (Variables|GameSettings|GetGameSettings)))))