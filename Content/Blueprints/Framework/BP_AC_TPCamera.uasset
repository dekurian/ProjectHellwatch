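; Third-person camera Blueprint that applies the player's graphics settings to its post-process effects.
; On BeginPlay it caches BP_GI_Main, binds to post-process setting updates and runs an initial refresh.
; Each refresh reads game settings to toggle separate post-process elements for motion blur, SSAO, lens flares, bloom and auto exposure.
; Anti-aliasing is exclusive: all modes are reset, then the selected None, Temporal AA or FXAA element is enabled.
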(event Custom|Update%20PPSettings
  (bind _gamesettings (Default|GetGameSettings (Variables|Default|GetGameInstance)))
  (Variables|/Script/Engine.PostProcessComponent|SetbEnabled (Variables|Default|GetPP_MotionBlur) (Default|GetPPMotionBlur _gamesettings))
  (Variables|/Script/Engine.PostProcessComponent|SetbEnabled (Variables|Default|GetPP_AmbientOcclusion) (Default|GetPPSSAO _gamesettings))
  (Variables|/Script/Engine.PostProcessComponent|SetbEnabled (Variables|Default|GetPP_LensFlares) (Default|GetPPLensflares _gamesettings))
  (Variables|/Script/Engine.PostProcessComponent|SetbEnabled (Variables|Default|GetPP_Bloom) (Default|GetPPBloom _gamesettings))
  (Variables|/Script/Engine.PostProcessComponent|SetbEnabled (Variables|Default|GetPP_AutoExposure) (Default|GetPPAutoExposure _gamesettings))
  (CallFunction|SetAAMethod (Default|GetAAMethod _gamesettings)))

(event EventBeginPlay
  (EventDispatchers|BindEventtoUpdatePostProcessSettings (delegate Custom|Update%20PPSettings))
  (bind _asbp_gi_main (Utilities|Casting|CastToBP_GI_Main (Game|GetGameInstance)))
  (Variables|Default|SetGameInstance _asbp_gi_main)
  (CallFunction|UpdatePPSettings))

(fn ConstructionScript)

(fn ResetAAMethod
  (Variables|/Script/Engine.PostProcessComponent|SetbEnabled (Variables|Default|GetPP_AA_TemporalAA) false)
  (Variables|/Script/Engine.PostProcessComponent|SetbEnabled (Variables|Default|GetPP_AA_FXAA) false)
  (Variables|/Script/Engine.PostProcessComponent|SetbEnabled (Variables|Default|GetPP_AA_None) false))

(fn SetAAMethod
  (params (AAMethod :type Integer))
  (CallFunction|ResetAAMethod)
  (switch int AAMethod
    (:0
      (Variables|/Script/Engine.PostProcessComponent|SetbEnabled (Variables|Default|GetPP_AA_None) true))
    (:1
      (Variables|/Script/Engine.PostProcessComponent|SetbEnabled (Variables|Default|GetPP_AA_TemporalAA) true))
    (:2
      (Variables|/Script/Engine.PostProcessComponent|SetbEnabled (Variables|Default|GetPP_AA_FXAA) true))))