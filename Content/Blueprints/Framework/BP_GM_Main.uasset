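; Main game mode that controls in-game cinematic sequences: run, pause, skip and end.
; RunSequence stores the sequence in BP_GS_Main, enters cinematic mode, freezes active AI and plays from the start with a length-based timer.
; EndSequence exits cinematic mode, blends the view back to the main character and restores AI walking.
; Pause toggles playback, timer and game pause, while Skip clears the timer, jumps to the end and calls EndSequence.
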(fn ConstructionScript)

(fn RunSequence
  (params (SequenceToBePlayed :type Level%20Sequence%20Actor%20Object%20Reference) (HidePlayerDuringSequence? :type Boolean) (CameraBlendSpeed :type Float%20%28single-precision%29))
  ;[1 1 1] Save Parameters
  (bind _output_get (LocalVariables|SetlocalSequence SequenceToBePlayed))
  (LocalVariables|SetlocalHidePlayer HidePlayerDuringSequence?)
  (LocalVariables|SetlocalCameraBlendSpeed CameraBlendSpeed)
  ;[1 1 1] First get the GameState since we need it here.
  (bind _asbp_gs_main (Utilities|Casting|CastToBP_GS_Main (Game|GetGameState)))
  (LocalVariables|SetlocalGameState _asbp_gs_main)
  ;[1 1 1] Init the Sequence and set the Position to 0, so we can trigger the Sequence again and again.
  (Default|SetSequenceInfo (LocalVariables|GetlocalGameState) true (LocalVariables|GetlocalSequence) (LocalVariables|GetlocalCameraBlendSpeed))
  (Components|Timeline|SetPlaybackPosition (Variables|/Script/LevelSequence.LevelSequenceActor|GetSequencePlayer _output_get) 0.0)
  (Class|PlayerController|SetCinematicMode (Game|GetPlayerController 0) true (LocalVariables|GetlocalHidePlayer) false true true)
  ;[1 1 1] Disable Movement of all AI
  (for _array_element (Variables|/Game/Blueprints/Framework/BP_GS_Main.BP_GS_Main_C|GetActiveAIActors (LocalVariables|GetlocalGameState))
    (Pawn|Components|CharacterMovement|DisableMovement (Variables|/Script/Engine.Character|GetCharacterMovement _array_element)))
  ;[1 1 1] Play the Actual Scene and specify the EndEvent.
  (Audio|Components|Audio|Play (Variables|/Script/LevelSequence.LevelSequenceActor|GetSequencePlayer (LocalVariables|GetlocalSequence)))
  (bind _returnvalue (Utilities|Time|SetTimerbyEvent (EventDispatchers|CreateEvent :!event EndSequence) (Class|LevelSequencePlayer|GetLength (Variables|/Script/LevelSequence.LevelSequenceActor|GetSequencePlayer (LocalVariables|GetlocalSequence)))))
  (Variables|/Game/Blueprints/Framework/BP_GS_Main.BP_GS_Main_C|SetHandleSequenceTimer (LocalVariables|GetlocalGameState) _returnvalue))

(fn EndSequence
  (bind _returnvalue (Game|GetPlayerController 0))
  ;[1 1 1] Save Reference to the GameState
  (bind _asbp_gs_main (Utilities|Casting|CastToBP_GS_Main (Game|GetGameState)))
  (LocalVariables|SetlocalGameState _asbp_gs_main)
  ;[1 1 1] End the Sequence
  (Class|PlayerController|SetCinematicMode _returnvalue false false true true true)
  (bind _asbp_ch_main_character (Utilities|Casting|CastToBP_CH_MainCharacter (Variables|/Game/Blueprints/Framework/BP_GS_Main.BP_GS_Main_C|GetMainPlayer (LocalVariables|GetlocalGameState))))
  (Game|Player|SetViewTargetwithBlend _returnvalue _asbp_ch_main_character (Variables|/Game/Blueprints/Framework/BP_GS_Main.BP_GS_Main_C|GetSequenceCameraBlendSpeed (LocalVariables|GetlocalGameState)) "VTBlend_Linear" 0.0 false)
  (Default|SetSequenceInfo (LocalVariables|GetlocalGameState) false 0 0.0)
  ;[1 1 1] Enable the Movement of the AI again.
  (for _array_element (Variables|/Game/Blueprints/Framework/BP_GS_Main.BP_GS_Main_C|GetActiveAIActors (LocalVariables|GetlocalGameState))
    (Pawn|Components|CharacterMovement|SetMovementMode (Variables|/Script/Engine.Character|GetCharacterMovement _array_element) "MOVE_Walking" 0)))

(fn PauseSequence
  ;[1 1 1] Get GameState reference.
  (bind _asbp_gs_main (Utilities|Casting|CastToBP_GS_Main (Game|GetGameState)))
  (bind _output_get (LocalVariables|SetlocalGameState _asbp_gs_main))
  ;[1 1 1] We need to know if the sequence is running or not.
  (if (Audio|Components|Audio|IsPlaying (Variables|/Script/LevelSequence.LevelSequenceActor|GetSequencePlayer (Variables|/Game/Blueprints/Framework/BP_GS_Main.BP_GS_Main_C|GetCurrentSequence _output_get)))
    ;[1 1 1] Pause the Sequence
    (Utilities|Time|PauseTimerbyHandle (Variables|/Game/Blueprints/Framework/BP_GS_Main.BP_GS_Main_C|GetHandleSequenceTimer (LocalVariables|GetlocalGameState)))
    (Sequencer|Player|Pause (Variables|/Script/LevelSequence.LevelSequenceActor|GetSequencePlayer (Variables|/Game/Blueprints/Framework/BP_GS_Main.BP_GS_Main_C|GetCurrentSequence _output_get)))
    (Game|SetGamePaused true)
    (else
      ;[1 1 1] Unpause the Sequence.
      (Utilities|Time|UnpauseTimerbyHandle (Variables|/Game/Blueprints/Framework/BP_GS_Main.BP_GS_Main_C|GetHandleSequenceTimer (LocalVariables|GetlocalGameState)))
      (Audio|Components|Audio|Play (Variables|/Script/LevelSequence.LevelSequenceActor|GetSequencePlayer (Variables|/Game/Blueprints/Framework/BP_GS_Main.BP_GS_Main_C|GetCurrentSequence _output_get)))
      (Game|SetGamePaused false))))

(fn SkipSequence
  (params (CameraBlendSpeed :type Float%20%28single-precision%29))
  ;[1 1 1] Save parameter.
  (LocalVariables|SetlocalCameraBlendSpeed CameraBlendSpeed)
  ;[1 1 1] Save reference to GameState.
  (bind _asbp_gs_main (Utilities|Casting|CastToBP_GS_Main (Game|GetGameState)))
  (bind _output_get (LocalVariables|SetlocalGameState _asbp_gs_main))
  ;[1 1 1] Set ne Blend Speed.
  (Default|SetSequenceInfo _output_get (Variables|/Game/Blueprints/Framework/BP_GS_Main.BP_GS_Main_C|GetIsInSequence _output_get) (Variables|/Game/Blueprints/Framework/BP_GS_Main.BP_GS_Main_C|GetCurrentSequence _output_get) (LocalVariables|GetlocalCameraBlendSpeed))
  ;[1 1 1] Set the Playback Position to the end of the current Sequence so we skip it and finish the rest.
  (Utilities|Time|ClearandInvalidateTimerbyHandle (Variables|/Game/Blueprints/Framework/BP_GS_Main.BP_GS_Main_C|GetHandleSequenceTimer (LocalVariables|GetlocalGameState)))
  (Components|Timeline|SetPlaybackPosition (Variables|/Script/LevelSequence.LevelSequenceActor|GetSequencePlayer (Variables|/Game/Blueprints/Framework/BP_GS_Main.BP_GS_Main_C|GetCurrentSequence (LocalVariables|GetlocalGameState))) (Class|LevelSequencePlayer|GetLength (Variables|/Script/LevelSequence.LevelSequenceActor|GetSequencePlayer (Variables|/Game/Blueprints/Framework/BP_GS_Main.BP_GS_Main_C|GetCurrentSequence (LocalVariables|GetlocalGameState)))))
  (CallFunction|EndSequence))