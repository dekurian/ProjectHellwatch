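; Main menu player controller that creates the menu widget and starts new, loaded or continued games.
; It relays GameMode menu state changes to the widget for transitions, and any key press advances from the initial title screen state.
; It stores save slot, difficulty and selection mode.
; New Game creates a save through the GameInstance; Load and Continue currently just open the same debug map as New Game.
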(event Custom|OnMenuStateChanged
  (params (FromState :type BPE_MainMenuState%20Enum) (ToState :type BPE_MainMenuState%20Enum))
  ;[1 1 1] Transition Handling Event
  (Default|HandleMenuTransition (Variables|MainMenu|GetMainMenu) FromState ToState))

(event EventBeginPlay
  ;[1 1 1] Save a Reference to the GameMode
  (bind _asbp_gm_main_menu (Utilities|Casting|CastToBP_GM_MainMenu (Game|GetGameMode)))
  (bind _output_get (Variables|Default|SetGameMode _asbp_gm_main_menu))
  ;[1 1 1] Bind the State-Change-Event
  (EventDispatchers|AssignOnMenuStateChanged _output_get (delegate Custom|OnMenuStateChanged))
  ;[1 1 1] Save a Reference to the Game Instance
  (bind _asbp_gi_main (Utilities|Casting|CastToBP_GI_Main (Game|GetGameInstance)))
  (Variables|Default|SetGameInstance _asbp_gi_main)
  ;[1 1 1] Create the Main-Menu, add it to the Viewport and save the Reference
  (Utilities|IsValid (Variables|MainMenu|GetMainMenu)
    (:Is%20Not%20Valid
      (bind _returnvalue (UserInterface|CreateWidget "/Game/UI/MainMenu/UI_MainMenu_00.UI_MainMenu_00_C"))
      (Variables|MainMenu|SetMainMenu _returnvalue)
      (UserInterface|Viewport|AddtoViewport (Variables|MainMenu|GetMainMenu) 0)
      (Default|SetMainMenuState (Variables|Default|GetGameMode) "NewEnumerator0")
      ;[1 1 1] Set the Input-Mode for the Title Screen
      (Input|SetInputModeGameOnly)
      (Variables|Default|SetbShowMouseCursor false))))

(event Input|KeyboardEvents|AnyKey
  (params (Key :type Key%20Structure :default "AnyKey"))
  ;[1 1 1] Input Title Screen
  (:Pressed
    (if (Utilities|Enum|Equal(Enum) (Default|GetMainMenuState (Variables|Default|GetGameMode)) "NewEnumerator0")
      (Default|SetMainMenuState (Variables|Default|GetGameMode) "NewEnumerator1"))))

(fn ConstructionScript)

(fn GetMainMenu
  (return (Variables|MainMenu|GetMainMenu)))

(fn SetSelectedSaveSlot
  (params (SaveSlot :type Integer))
  (Variables|MainMenu|SetSelectedSaveSlot SaveSlot))

(fn SetSelectedGameDifficulty
  (params (GameDifficulty :type BPE_GameDifficulty%20Enum))
  (Variables|MainMenu|SetSelectedGameDifficulty GameDifficulty))

(fn SetSaveSlotSelectionMode
  (params (Mode :type BPE_SaveSelectionMode%20Enum))
  (Variables|MainMenu|SetSaveSlotSelectionMode Mode))

(fn GetSaveSlotSelectionMode
  (return (Variables|MainMenu|GetSaveSlotSelectionMode)))

(fn InitNewGame
  (Default|CreateNewSaveGame (Variables|Default|GetGameInstance) (Variables|MainMenu|GetSelectedSaveSlot) (Variables|MainMenu|GetSelectedGameDifficulty))
  (Game|OpenLevel(byName) "MAP_Debug_01"))

(fn InitLoadGame
  (Game|OpenLevel(byName) "MAP_Debug_01"))

(fn InitContinue
  (Game|OpenLevel(byName) "MAP_Debug_01"))